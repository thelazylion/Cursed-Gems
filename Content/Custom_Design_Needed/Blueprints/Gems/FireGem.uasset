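; FireGem is a pickup that grants the third-person character fire status and triggers level changes.
; A timeline started on BeginPlay animates the sphere with relative height offsets and randomized rotation on every update.
; When the character overlaps it, the gem sets Firey, spawns a large Lava actor at a hard-coded transform, destroys itself, then plays the first-door-up level sequence.
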(event `self.ReceiveBeginPlay`
  (bind (_direction _height _rot) (`Timeline|Gem Motion`)
    (:`Update`
      (`SceneComponent.K2_AddRelativeLocation` (`self.Sphere`) (`KismetMathLibrary.MakeVector` 0.0 0.0 _height) false false)
      (bind _returnvalue (`KismetMathLibrary.RandomFloatInRange` _height _rot))
      (`SceneComponent.K2_AddRelativeRotation` (`self.Sphere`) (`KismetMathLibrary.MakeRotator` _returnvalue _returnvalue _returnvalue) false false))))

(event `self.ReceiveActorBeginOverlap`
  (params (OtherActor :type "Actor Object Reference"))
  (bind _asthird_person_character (cast `/Game/ThirdPersonBP/Blueprints/ThirdPersonCharacter` OtherActor))
  (set `/Game/ThirdPersonBP/Blueprints/ThirdPersonCharacter.Firey` true _asthird_person_character)
  (`|SpawnActorFromClass` "/Game/Custom_Design_Needed/Blueprints/Lava.Lava_C" (`KismetMathLibrary.MakeTransform` (24148.0 5943.0 -1819.0) (struct :`Yaw` 45.0) (50.0 50.0 1.0)) "Undefined" "OverrideRootScale" null null)
  (`self.K2_DestroyActor`)
  (bind _outactor (`LevelSequencePlayer.CreateLevelSequencePlayer` "/Game/Custom_Design_Needed/Cinematics/Level1/1stDoor_Up_Sequence.1stDoor_Up_Sequence"))
  (`MovieSceneSequencePlayer.Play` (`LevelSequenceActor.SequencePlayer` _outactor)))

(fn `UserConstructionScript`)