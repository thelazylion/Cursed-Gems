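; IceGem is a pickup actor that gives the ThirdPersonCharacter icy movement when overlapped.
; On overlap it overwrites the character's movement settings for acceleration, ground friction, braking and walk speed, sets its Icy flag, then destroys itself without any revert logic.
; The construction script creates a dynamic instance of Lava_MAT on the Sphere and tints its emissive color light blue.
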(event `self.ReceiveActorBeginOverlap`
  (params (OtherActor :type "Actor Object Reference"))
  (bind _asthird_person_character (cast `/Game/ThirdPersonBP/Blueprints/ThirdPersonCharacter` OtherActor))
  (bind _charactermovement (`Character.CharacterMovement` _asthird_person_character))
  (set `CharacterMovementComponent.MaxAcceleration` 1024.0 _charactermovement)
  (set `CharacterMovementComponent.GroundFriction` 0.25 _charactermovement)
  (set `CharacterMovementComponent.BrakingFrictionFactor` 1.0 _charactermovement)
  (set `CharacterMovementComponent.BrakingDecelerationWalking` 512.0 _charactermovement)
  (set `CharacterMovementComponent.MaxWalkSpeed` 1024.0 _charactermovement)
  (set `/Game/ThirdPersonBP/Blueprints/ThirdPersonCharacter.Icy` true _asthird_person_character)
  (`self.K2_DestroyActor`))

(fn `UserConstructionScript`
  (bind _returnvalue (`PrimitiveComponent.CreateDynamicMaterialInstance` (`self.Sphere`) 0 "/Game/StarterContent/Textures/Lava_MAT.Lava_MAT"))
  (`MaterialInstanceDynamic.SetVectorParameterValue` _returnvalue "EmissColor" (struct :`G` 0.621619 :`B` 1.0 :`A` 1.0)))