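; Lava actor that raises its plane mesh vertically once play begins.
; BeginPlay starts the Lavarise timeline from the beginning, and each update writes its Rise track to the plane's relative Z location.
; Disconnected leftover nodes sketch a Glowflow timeline driving a Substance warp-angle input with async rendering, but they never run.
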(event `self.ReceiveBeginPlay`
  (bind (_direction _rise) (`Timeline|lavarise` :!via `PlayFromStart`)
    (:`Update`
      (`SceneComponent.K2_SetRelativeLocation` (`self.Plane`) (`KismetMathLibrary.MakeVector` 0.0 0.0 _rise) false false))))

(event `self.ReceiveTick`
  (params (DeltaSeconds :type "Float (single-precision)")))

(fn `UserConstructionScript`)