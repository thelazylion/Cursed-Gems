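; FlameProjectile is a projectile actor, a flame by its name, that changes speed over time and removes itself.
; A timeline started on BeginPlay repeatedly multiplies the movement component's current modified max speed into MaxSpeed, so scaling compounds, and feeds a six-second delay before destruction.
; Capsule overlap destroys it only when the other actor is itself, so hits on other actors do nothing.
; Random rotation logic is present but unconnected.
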(event `self.ReceiveBeginPlay`
  (bind _projectilemovement (`self.ProjectileMovement`))
  (bind (_direction _newtrack_0) (`Timeline|Timeline_0` :!via `PlayFromStart`)
    (:`Update`
      (set `ProjectileMovementComponent.MaxSpeed` (* _newtrack_0 (`MovementComponent.K2_GetModifiedMaxSpeed` _projectilemovement)) _projectilemovement)
      (`KismetSystemLibrary.Delay` 6.0)
      (`self.K2_DestroyActor`))))

(event `self.Capsule.OnComponentBeginOverlap`
  (params (OverlappedComponent :type "PrimitiveComponent Object Reference") (OtherActor :type "Actor Object Reference") (OtherComp :type "PrimitiveComponent Object Reference") (OtherBodyIndex :type Integer) (bFromSweep :type Boolean) (SweepResult :type "HitResult Structure (by ref)"))
  (if (not (!= OtherActor self))
    (`self.K2_DestroyActor`)))

(fn `UserConstructionScript`)