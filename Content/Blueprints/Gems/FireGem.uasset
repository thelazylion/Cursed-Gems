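; FireGem is a gem pickup that spawns Lava when the ThirdPersonCharacter touches it.
; On BeginPlay the GemMotion timeline moves the Sphere along Z and adds random rotation on each axis, bounded by its Height and Rot tracks.
; On a character overlap it spawns a very wide Lava actor at a fixed world location, then destroys itself.
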(event `self.ReceiveBeginPlay`
  (bind (_direction _height _rot) (`Timeline|Gem Motion`)
    (:`Update`
      (`SceneComponent.K2_AddRelativeLocation` (`self.Sphere`) (`KismetMathLibrary.MakeVector` 0.0 0.0 _height) false false)
      (bind _returnvalue (`KismetMathLibrary.RandomFloatInRange` _height _rot))
      (`SceneComponent.K2_AddRelativeRotation` (`self.Sphere`) (`KismetMathLibrary.MakeRotator` _returnvalue _returnvalue _returnvalue) false false))))

(event `self.ReceiveActorBeginOverlap`
  (params (OtherActor :type "Actor Object Reference"))
  (cast `/Game/ThirdPersonBP/Blueprints/ThirdPersonCharacter` OtherActor)
  (`|SpawnActorFromClass` "/Game/Blueprints/Lava.Lava_C" (`KismetMathLibrary.MakeTransform` (-2000.0 0.0 0.0) (struct) (210.0 210.0 1.0)) "Undefined" "OverrideRootScale" null null)
  (`self.K2_DestroyActor`))

(fn `UserConstructionScript`)